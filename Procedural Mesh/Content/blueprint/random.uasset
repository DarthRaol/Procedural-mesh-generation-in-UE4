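; Short-lived radial force actor that fires one impulse on spawn and destroys itself when its timeline finishes.
; While playing, the timeline drives the RadialForce component's continuous force strength.
; The X key flip-flops impulse and force strength between negative (pull) and positive (push), though timeline updates overwrite the force value.
; The looping implosion timer and overlap-destroy nodes are disconnected.
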(event `self.ReceiveBeginPlay`
  (`RadialForceComponent.FireImpulse` (`self.RadialForce`))
  (bind (_direction _newtrack_0) (`Timeline|Timeline_0`)
    (:`Update`
      (set `RadialForceComponent.ForceStrength` _newtrack_0 (`self.RadialForce`)))
    (:`Finished`
      (`self.K2_DestroyActor`))))

(event `self.ReceiveTick`
  (params (DeltaSeconds :type "Float (single-precision)")))

(event `Key|X`
  (params (Key :type "Key Structure"))
  (bind _radialforce (`self.RadialForce`))
  (:`Pressed`
    (`/Engine/EditorBlueprintResources/StandardMacros.FlipFlop`
      (:`A`
        (set `RadialForceComponent.ImpulseStrength` -10.0 _radialforce)
        (set `RadialForceComponent.ForceStrength` -100000.0 _radialforce))
      (:`B`
        (set `RadialForceComponent.ImpulseStrength` 10.0 _radialforce)
        (set `RadialForceComponent.ForceStrength` 100000.0 _radialforce)))))

(event `self.Sphere.OnComponentBeginOverlap`
  (params (OverlappedComponent :type "PrimitiveComponent Object Reference") (OtherActor :type "Actor Object Reference") (OtherComp :type "PrimitiveComponent Object Reference") (OtherBodyIndex :type Integer) (bFromSweep :type Boolean) (SweepResult :type "HitResult Structure (by ref)")))

(fn `implosion`
  (`RadialForceComponent.FireImpulse` (`self.RadialForce`)))

(fn `UserConstructionScript`)