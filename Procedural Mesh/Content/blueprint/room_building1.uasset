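; Procedural modular building actor that assembles a box-shaped building from static meshes in its Construction Script.
; Nested length, breadth and height loops classify each grid cell as corner or edge, using roof variants, plus a center piece, on the top layer.
; An optional interior mesh fills every cell.
; A helper adds each mesh component at index times module size, picking a variant from its array via a random stream.
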(event `self.ReceiveTick`
  (params (DeltaSeconds :type "Float (single-precision)")))

(fn `spawn mesh at co_ordinates`
  (params (`static mesh Array` :type "Array of StaticMesh Object Reference"))
  (bind _length_of_static_mesh (`self.length of static mesh`))
  (bind _returnvalue (`AddComponent|NODE_AddStaticMeshComponent-12` :`RelativeTransform` (`KismetMathLibrary.MakeTransform` (`KismetMathLibrary.MakeVector` (* (`self.index_of_length`) _length_of_static_mesh) (* (`self.index_of_breadth`) _length_of_static_mesh) (* (`self.index_of_height`) _length_of_static_mesh)))))
  (`StaticMeshComponent.SetStaticMesh` _returnvalue (`|GetArrayItem` `static mesh Array` (`KismetMathLibrary.RandomIntegerInRangeFromStream` 0 (- (`KismetArrayLibrary.Array_Length` `static mesh Array`) 1) (`self.stream`)))))

(fn `UserConstructionScript`
  (bind _index_of_breadth (`self.index_of_breadth`))
  (bind _index_of_breadth_2 (`self.index_of_breadth`))
  (bind _index_of_breadth_3 (`self.index_of_breadth`))
  (bind _index_of_length (`self.index_of_length`))
  (bind _index_of_length_2 (`self.index_of_length`))
  (bind _index_of_length_3 (`self.index_of_length`))
  (bind _index_of_length_4 (`self.index_of_length`))
  (bind _index_of_breadth_4 (`self.index_of_breadth`))
  ;[1 1 1] initialization
  (if (!= (`self.breadth`) (`self.index_of_breadth`))
    (for _index (range (+ (`self.lenght`) 1)) :!label _label
      (set `self.index_of_length` _index)
      (for _index_2 (range (+ (`self.breadth`) 1))
        (set `self.index_of_breadth` _index_2)
        (for _index_3 (range (+ (`self.height`) 1))
          (set `self.index_of_height` _index_3)
          ;[1 1 1] enable interior and roof setup
          (if (`self.Enable_interior_build`)
            (`self.spawn mesh at co_ordinates` (`self.static-mesh_int`)))
          (if (== (`self.index_of_height`) (`self.height`))
            ;[1 1 1] roof setup
            (if (and (== (`self.index_of_length`) 0) (== 0 (`self.index_of_breadth`)))
              (`self.spawn mesh at co_ordinates` (`self.SM_roof_0_0`))
              (elif (and (== (`self.index_of_length`) (`self.lenght`)) (== (`self.breadth`) (`self.index_of_breadth`)))
                (`self.spawn mesh at co_ordinates` (`self.SM_roof_L_L`))
                (elif (and (== (`self.index_of_length`) 0) (== (`self.breadth`) (`self.index_of_breadth`)))
                  (`self.spawn mesh at co_ordinates` (`self.SM_roof_0_L`))
                  (elif (and (== (`self.index_of_length`) (`self.lenght`)) (== 0 (`self.index_of_breadth`)))
                    (`self.spawn mesh at co_ordinates` (`self.SM_roof_L_0`))
                    (elif (and (== (`self.index_of_length`) 0) (!= 0 _index_of_breadth_2) (!= _index_of_breadth_2 (`self.breadth`)))
                      (`self.spawn mesh at co_ordinates` (`self.SM_roof_edge_1`))
                      (elif (and (== (`self.index_of_breadth`) 0) (!= _index_of_length_2 0) (!= _index_of_length_2 (`self.lenght`)))
                        (`self.spawn mesh at co_ordinates` (`self.SM_roof_edge_2`))
                        (elif (and (== (`self.index_of_breadth`) (`self.breadth`)) (!= _index_of_length_3 0) (!= _index_of_length_3 (`self.lenght`)))
                          (`self.spawn mesh at co_ordinates` (`self.SM_roof_edge_3`))
                          (elif (and (== (`self.index_of_length`) (`self.lenght`)) (!= _index_of_breadth 0) (!= _index_of_breadth (`self.breadth`)))
                            (`self.spawn mesh at co_ordinates` (`self.SM_roof_edge_4`))
                            (else
                              (`self.spawn mesh at co_ordinates` (`self.SM_roof_center`)))))))))))
            (elif (and (== (`self.index_of_length`) 0) (== 0 (`self.index_of_breadth`)))
              (`self.spawn mesh at co_ordinates` (`self.static_mesh_0_0`))
              (elif (and (== (`self.index_of_length`) (`self.lenght`)) (== (`self.breadth`) (`self.index_of_breadth`)))
                (`self.spawn mesh at co_ordinates` (`self.static_mesh_L_L`))
                (elif (and (== (`self.index_of_length`) 0) (== (`self.breadth`) (`self.index_of_breadth`)))
                  (`self.spawn mesh at co_ordinates` (`self.static_mesh_0_L`))
                  (elif (and (== (`self.index_of_length`) (`self.lenght`)) (== 0 (`self.index_of_breadth`)))
                    (`self.spawn mesh at co_ordinates` (`self.static_mesh_L_0`))
                    (elif (and (== (`self.index_of_length`) 0) (!= 0 _index_of_breadth_3) (!= _index_of_breadth_3 (`self.breadth`)))
                      (`self.spawn mesh at co_ordinates` (`self.static_mesh_edge_1`))
                      (elif (and (== (`self.index_of_breadth`) 0) (!= _index_of_length 0) (!= _index_of_length (`self.lenght`)))
                        (`self.spawn mesh at co_ordinates` (`self.static_mesh_edge_2`))
                        (elif (and (== (`self.index_of_breadth`) (`self.breadth`)) (!= _index_of_length_4 0) (!= _index_of_length_4 (`self.lenght`)))
                          (`self.spawn mesh at co_ordinates` (`self.static_mesh_edge_3`))
                          (elif (and (== (`self.index_of_length`) (`self.lenght`)) (!= _index_of_breadth_4 0) (!= _index_of_breadth_4 (`self.breadth`)))
                            (`self.spawn mesh at co_ordinates` (`self.static_mesh_edge_4`))))))))))))))
    (else
      (goto _label :!via `Break`))))