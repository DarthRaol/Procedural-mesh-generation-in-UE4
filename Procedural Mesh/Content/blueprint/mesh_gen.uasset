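; Procedural mesh actor that generates a grid surface with noisy height, built in the construction script whenever the Update flag is toggled on.
; AddVertices lays out grid points and normalized UVs, with height from 1D Perlin noise of a random input, so neighboring heights are uncorrelated.
; AddTriangles inserts quad indices at positions read from the Triangle array itself, advancing seven per quad.
; The arrays feed one mesh section with collision.
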(fn `Add triangles`
  (bind _triangle (`self.triangle`))
  (bind _triangle_2 (`self.triangle`))
  (bind _triangle_3 (`self.triangle`))
  (bind _triangle_4 (`self.triangle`))
  (bind _triangle_5 (`self.triangle`))
  (bind _triangle_6 (`self.triangle`))
  (set `self.vert` 0)
  (set `self.tris` 0)
  (for _ (range (+ (`self.Y_size`) 1))
    (for _ (range (+ (`self.X_size`) 1))
      (`KismetArrayLibrary.Array_Insert` _triangle_5 (+ (`self.vert`) 0) (`|GetArrayItem` _triangle_5 (+ (`self.tris`) 0)))
      (`KismetArrayLibrary.Array_Insert` _triangle_6 (+ (`self.vert`) 1 (`self.X_size`)) (`|GetArrayItem` _triangle_6 (+ (`self.tris`) 1)))
      (`KismetArrayLibrary.Array_Insert` _triangle_2 (+ (`self.vert`) 1) (`|GetArrayItem` _triangle_2 (+ (`self.tris`) 2)))
      (`KismetArrayLibrary.Array_Insert` _triangle_3 (+ (`self.vert`) 1) (`|GetArrayItem` _triangle_3 (+ (`self.tris`) 3)))
      (`KismetArrayLibrary.Array_Insert` _triangle_4 (+ (`self.vert`) (`self.X_size`) 1) (`|GetArrayItem` _triangle_4 (+ (`self.tris`) 4)))
      (`KismetArrayLibrary.Array_Insert` _triangle (+ (`self.vert`) 2 (`self.X_size`)) (`|GetArrayItem` _triangle (+ (`self.tris`) 5)))
      (set `self.vert` (+ (`self.vert`) 1))
      (set `self.tris` (+ (`self.tris`) 7)))))

(fn `Add vertices`
  (params (X_size :type Integer) (Y_size :type Integer) (vertices :type "Array of Vector Structure (by ref)") (UV_0 :type "Array of Vector2D Structure (by ref)"))
  (set `self.time` 0.0)
  (for _index (range (+ X_size 1))
    (bind _output_get (set `self.X` _index))
    (for _index_2 (range (+ Y_size 1))
      (bind _output_get_2 (set `self.y` _index_2))
      (set `self.time` (+ (`self.time`) 0.1))
      (bind _returnvalue (`KismetMathLibrary.Conv_IntToDouble` _output_get))
      (bind _returnvalue_2 (`KismetMathLibrary.Conv_IntToDouble` _output_get_2))
      (`KismetArrayLibrary.Array_Add` vertices (`KismetMathLibrary.MakeVector` _returnvalue _returnvalue_2 (* 1 (`KismetMathLibrary.PerlinNoise1D` (`KismetMathLibrary.RandomFloatInRange` -2.0 2.0)))))
      (`KismetArrayLibrary.Array_Add` UV_0 (`KismetMathLibrary.MakeVector2D` (/ _returnvalue (`KismetMathLibrary.Conv_IntToDouble` (`self.X_size`))) (/ _returnvalue_2 (`KismetMathLibrary.Conv_IntToDouble` (`self.Y_size`))))))))

(fn `UserConstructionScript`
  (bind _vertices (`self.vertices`))
  (bind _uv_0 (`self.UV_0`))
  (if (`self.update`)
    (set `self.update` false)
    (`self.Add vertices` (`self.X_size`) (`self.Y_size`) _vertices _uv_0)
    (`self.Add triangles`)
    (`ProceduralMeshComponent.CreateMeshSection_LinearColor` :`self` (`self.ProceduralMesh`) :`Vertices` _vertices :`Triangles` (`self.triangle`) :`UV0` _uv_0 :`bCreateCollision` true)))